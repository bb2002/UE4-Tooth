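; BP_GamePawn is the player pawn for ToothGame, with a VR camera rig and a widget component that shows the player toast.
; It exposes helper functions to fetch the PlayerToast widget, read the camera's world rotation and hide the toast.
; A downward visibility trace from the VR camera root supplies the bottom location, returned without checking for a hit.
; The event graph and construction script contain no logic.
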(fn `DisableToast`
  (`SceneComponent.SetVisibility` (`self.Widget`) false false))

(fn `GetBottomLocation`
  (returns (NewParam :type "Vector Structure"))
  (bind _vrcameraroot (`self.VRCameraRoot`))
  (bind _outhit (`KismetSystemLibrary.LineTraceSingle` (`SceneComponent.K2_GetComponentLocation` _vrcameraroot) (`KismetMathLibrary.MakeVector` (.x (`SceneComponent.K2_GetComponentLocation` _vrcameraroot)) (.y (`SceneComponent.K2_GetComponentLocation` _vrcameraroot)) (* (.z (`SceneComponent.K2_GetComponentLocation` _vrcameraroot)) -100.0)) "TraceTypeQuery1"))
  (if true
    (return (`.Location` (`GameplayStatics.BreakHitResult` _outhit)))))

(fn `GetPlayerRotation`
  (returns (Rotation :type "Rotator Structure"))
  (return (`SceneComponent.K2_GetComponentRotation` (`self.CameraComponent`))))

(fn `GetPlayerToast`
  (returns (NewParam :type "/Game/ToothGame/Game/UI/Stage/PlayerToast Object Reference"))
  (bind _asplayer_toast (cast `/Game/ToothGame/Game/UI/Stage/PlayerToast` (`WidgetComponent.GetUserWidgetObject` (`self.Widget`))))
  (return _asplayer_toast))

(fn `UserConstructionScript`)